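; Tank pawn Blueprint whose graph only handles toggling the pause menu.
; P and Escape share one branch on IsPauseMenuOpen.
; Opening creates WB_PauseMenu, pauses the game, switches to UI-only input and shows the cursor.
; Closing removes the widget and unpauses, but does not restore the input mode or hide the cursor.
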(event `Key|P`
  (params (Key :type "Key Structure"))
  (bind _returnvalue (`GameplayStatics.GetPlayerController` 0))
  (:`Pressed`
    (if (not (`self.isPauseMenuOpen`)) :!label _label
      (set `self.isPauseMenuOpen` true)
      (bind _returnvalue_2 (`|CreateWidget` "/Game/UI/WB_PauseMenu.WB_PauseMenu_C" _returnvalue))
      (bind _output_get (set `self.Pause Menu Widget` _returnvalue_2))
      (`UserWidget.AddToViewport` _output_get 0)
      (`GameplayStatics.SetGamePaused` true)
      (`WidgetBlueprintLibrary.SetInputMode_UIOnlyEx` null null)
      (set `PlayerController.bShowMouseCursor` true _returnvalue)
      (else
        (set `self.isPauseMenuOpen` false)
        (`Widget.RemoveFromParent` (`self.Pause Menu Widget`))
        (`GameplayStatics.SetGamePaused` false)))))

(event `Key|Escape` :paused true
  (params (Key :type "Key Structure"))
  (:`Pressed`
    (goto _label)))

(fn `UserConstructionScript`
  (`parent.UserConstructionScript`))
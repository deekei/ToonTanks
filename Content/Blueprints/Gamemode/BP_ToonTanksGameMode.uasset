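; Game mode Blueprint for Toon Tanks that puts up the UI for the start, play and end phases of a match.
; StartGame and DuringGame add the start and HUD widgets only when the current level is Level1.
; GameOver shows the end-game widget with win or loss text from its WonGame flag.
; The mouse-cursor node is unconnected, and CheckLevelType tests the level name without producing any result.
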(event `self.GameOver`
  (params (bWonGame :type Boolean))
  (bind _returnvalue (`|CreateWidget` "/Game/Blueprints/Widgets/WBP_EndGameWidget.WBP_EndGameWidget_C"))
  (`UserWidget.AddToViewport` _returnvalue 0)
  (`TextBlock.SetText` (`/Game/Blueprints/Widgets/WBP_EndGameWidget.DisplayText` _returnvalue) (select `bool` bWonGame :`false` "Game Over!!" :`true` "You Won!" :!type "Text")))

(event `self.DuringGame`
  (bind _returnvalue (`GameplayStatics.GetCurrentLevelName` true))
  (if (`KismetStringLibrary.EqualEqual_StrStr` _returnvalue (`self.Level1`))
    (bind _returnvalue_2 (`|CreateWidget` "/Game/Blueprints/Widgets/WBP_HUDWidget.WBP_HUDWidget_C"))
    (`UserWidget.AddToViewport` _returnvalue_2 0)))

(event `self.StartGame`
  (bind _returnvalue (`GameplayStatics.GetCurrentLevelName` true))
  (if (`KismetStringLibrary.EqualEqual_StrStr` _returnvalue (`self.Level1`))
    (bind _returnvalue_2 (`|CreateWidget` "/Game/Blueprints/Widgets/WBP_StartGameWidget.WBP_StartGameWidget_C"))
    (`UserWidget.AddToViewport` _returnvalue_2 0)))

(fn `Check Level Type`
  (bind _returnvalue (`GameplayStatics.GetCurrentLevelName` true))
  (if (`KismetStringLibrary.EqualEqual_StrStr` _returnvalue (`self.Level1`))
    (return)))

(fn `UserConstructionScript`)